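; Hover physics test Blueprint that applies upward impulses at three points: front, back left and back right.
; Releasing W, Q or E fires a fixed-strength impulse at the matching Impulser component's location.
; Each location is the component's RelativeLocation, passed directly to AddImpulseAtLocation without conversion to world space.
; There is no continuous hover logic, as Tick and the construction script are empty.
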(event `self.ReceiveBeginPlay`)

(event `self.ReceiveActorBeginOverlap`
  (params (OtherActor :type "Actor Object Reference")))

(event `self.ReceiveTick`
  (params (DeltaSeconds :type "Float (single-precision)")))

(event `Key|W`
  (:`Released`
    (`PrimitiveComponent.AddImpulseAtLocation` (0.0 0.0 2000.0) (`SceneComponent.RelativeLocation` (`self.FrontImpulser`)))))

(event `Key|Q`
  (:`Released`
    (`PrimitiveComponent.AddImpulseAtLocation` (0.0 0.0 2000.0) (`SceneComponent.RelativeLocation` (`self.BackLeftImpulser`)))))

(event `Key|E`
  (:`Released`
    (`PrimitiveComponent.AddImpulseAtLocation` (0.0 0.0 2000.0) (`SceneComponent.RelativeLocation` (`self.BackRightImpulser`)))))

(fn `UserConstructionScript`)